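; BP_ExplodeComponent is the Collaborative Viewer's explode command, exposing an "Execute" option for each BP_Explode actor in the level.
; BeginPlay gathers those actors, and ExecuteAfterSpawnPawn builds a contextual button for each, named after the actor and bound to its array index.
; A press routes through StartAnim_ROS to StartAnim_MTC, apparently a server-to-multicast relay, which calls ExplodeAnim on that actor.
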(event `self.ExecuteAfterSpawnPawn`
  ;[0 1 0.1488] BeginPlayAfterSpawn
  (set `self.OptionsButtonNames` (`|MakeArray` "Execute" :!type "Text"))
  (for (_array_element _array_index) (`self.ExplodeData`)
    (set `self.Name` (`KismetTextLibrary.Conv_StringToText` (`KismetSystemLibrary.GetDisplayName` _array_element)))
    (`self.CreateContextualButon`)
    (`self.Bind_Option_Desktop` _array_index)
    (`KismetArrayLibrary.Array_Clear` (`self.OptionsButtons`))))

(event `self.ReceiveBeginPlay`
  ;[0 1 0.1488] BeginPlayAfterSpawn
  (bind _outactors (`GameplayStatics.GetAllActorsOfClass` "/Game/CollaborativeViewer/Blueprints/Commands/Explode/BP_Explode.BP_Explode_C"))
  (set `self.ExplodeData` _outactors))

(event `StartAnim_MTC`
  (params (id :type Integer))
  ;[0.3384 0.6313 1] Animation
  (`/Game/CollaborativeViewer/Blueprints/Commands/Explode/BP_Explode.Explode_Anim` (`|GetArrayItem` (`self.ExplodeData`) id)))

(event `StartAnim_ROS`
  (params (id :type Integer))
  ;[0.3384 0.6313 1] Animation
  (`self.StartAnim_MTC` id))

(event `Bind_Option_Desktop`
  (params (id :type Integer))
  (bind _output (`|GetArrayItem` (`self.OptionsButtons`)))
  ;[0.3384 0.6313 1] Setup Option Buttons
  (set `/Game/CollaborativeViewer/UMG/GameMenu/Option_Button.WhenExecute` "NewEnumerator1" _output)
  (set `/Game/CollaborativeViewer/UMG/GameMenu/Option_Button.id` id _output)
  (add `/Game/CollaborativeViewer/UMG/GameMenu/Option_Button.Execute` _output (delegate `Option1`)))

(event `Option1`
  (params (id :type Integer))
  ;[0.3384 0.6313 1] Setup Option Buttons
  (`self.StartAnim_ROS` id))