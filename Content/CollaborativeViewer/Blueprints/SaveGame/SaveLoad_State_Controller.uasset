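; Controller-side save/load manager for Collaborative Viewer states, linking the persistent UI's save and load controls to the player pawn.
; On its one-time startup it loads or creates a main save game that indexes slot names, then fills the load menu from it.
; It binds to the UI's save and load events and has handlers that delegate saving and loading to the pawn's SaveLoad_State_Pawn component.
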(event `BeginPlayFromController`
  (`/Engine/EditorBlueprintResources/StandardMacros.DoOnce` false
    (:`Completed`
      (bind _asbp_collab_v_player_controller (cast `/Game/CollaborativeViewer/Blueprints/PlayerController/BP_Collab_V_PlayerController` (`GameplayStatics.GetPlayerController` 0)))
      (set `self.Persistent_UI` (`/Game/CollaborativeViewer/Blueprints/PlayerController/BP_Collab_V_PlayerController.Persistent_UI` _asbp_collab_v_player_controller))
      (`self.CreateMainSlot_SaveGame`)
      (`self.MainSaveGameToPersistentMenu`)
      (`self.BindToMenu`))))

(event `BindToMenu`
  (bind _asbp_collab_v_player_controller (cast `/Game/CollaborativeViewer/Blueprints/PlayerController/BP_Collab_V_PlayerController` (`GameplayStatics.GetPlayerController` 0)))
  (bind _persistent_ui (`/Game/CollaborativeViewer/Blueprints/PlayerController/BP_Collab_V_PlayerController.Persistent_UI` _asbp_collab_v_player_controller))
  (add `/Game/CollaborativeViewer/UMG/GameMenu/Persistent_ToolBar.SavingState` _persistent_ui (`|CreateDelegate` :!event `AddToMainSveGame`))
  (add `/Game/CollaborativeViewer/UMG/GameMenu/Persistent_ToolBar.LoadState` _persistent_ui (`|CreateDelegate` :!event `LoadSaveGame`)))

(event `AddToMainSveGame`
  (params (SlotName :type "String (by ref)"))
  (`/Game/CollaborativeViewer/Blueprints/SaveGame/SaveLoad_State_Pawn.SaveGameROS` (`Actor.GetComponentByClass` (`GameplayStatics.GetPlayerPawn` 0) "/Game/CollaborativeViewer/Blueprints/SaveGame/SaveLoad_State_Pawn.SaveLoad_State_Pawn_C") SlotName (`self.SaveGame`)))

(event `LoadSaveGame`
  (params (Option :type String) (SaveGameMain :type "/Game/CollaborativeViewer/Blueprints/SaveGame/BP_Data_SaveGame Object Reference"))
  (`/Game/CollaborativeViewer/Blueprints/SaveGame/SaveLoad_State_Pawn.LoadSaveGameROS` (`Actor.GetComponentByClass` (`GameplayStatics.GetPlayerPawn` 0) "/Game/CollaborativeViewer/Blueprints/SaveGame/SaveLoad_State_Pawn.SaveLoad_State_Pawn_C") Option SaveGameMain))

(event `MainSaveGameToPersistentMenu`
  (bind _persistent_ui (`/Game/CollaborativeViewer/Blueprints/PlayerController/BP_Collab_V_PlayerController.Persistent_UI` (cast `/Game/CollaborativeViewer/Blueprints/PlayerController/BP_Collab_V_PlayerController` (`GameplayStatics.GetPlayerController` 0) :!pure true)))
  (`/Engine/EditorBlueprintResources/StandardMacros.IsValid` _persistent_ui
    (:`Is Valid`
      (for _array_element (`/Game/CollaborativeViewer/Blueprints/SaveGame/BP_Name_SaveGame.SaveGameNameArray` (`self.SaveGame`))
        (`ComboBoxString.AddOption` (`/Game/CollaborativeViewer/UMG/GameMenu/Persistent_ToolBar.Load_State` _persistent_ui) _array_element)))))

(event `CreateMainSlot_SaveGame`
  (if (`BlueprintPathsLibrary.FileExists` (`KismetStringLibrary.Concat_StrStr` (`KismetSystemLibrary.GetProjectSavedDirectory`) "SaveGames/MainSaveGame.sav"))
    (bind _returnvalue (`GameplayStatics.LoadGameFromSlot` "MainSaveGame"))
    (bind _asbp_name_save_game (cast `/Game/CollaborativeViewer/Blueprints/SaveGame/BP_Name_SaveGame` _returnvalue))
    (set `self.SaveGame` _asbp_name_save_game)
    (else
      (bind _returnvalue_2 (`GameplayStatics.CreateSaveGameObject` "/Game/CollaborativeViewer/Blueprints/SaveGame/BP_Name_SaveGame.BP_Name_SaveGame_C"))
      (set `self.SaveGame` _returnvalue_2)
      (bind _returnvalue_3 (`GameplayStatics.CreateSaveGameObject` "/Game/CollaborativeViewer/Blueprints/SaveGame/BP_Data_SaveGame.BP_Data_SaveGame_C"))
      (`GameplayStatics.SaveGameToSlot` _returnvalue_3 (`ComboBoxString.GetOptionAtIndex` (`/Game/CollaborativeViewer/UMG/GameMenu/Persistent_ToolBar.Load_State` (`self.Persistent_UI`)) 0)))))