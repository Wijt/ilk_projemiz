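; Laser pointer actor for the Collaborative Viewer, drawn between a start point and a hit location.
; UpdateLaser stores endpoints from an offset camera or supplied position and the hit, collapsing to the start without a blocking hit.
; SetLaserMesh aims and stretches LaserScaleRoot between two points, while UpdateOnServer stores received endpoints.
; The chain linking these steps is disconnected, the OnRep is empty, and Tick only prints local-control debug text.
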(event `self.ReceiveBeginPlay`)

(event `self.ReceiveTick`
  (params (DeltaSeconds :type "Float (single-precision)"))
  (if (`self.IsLocallyControlled` (`GameplayStatics.GetPlayerPawn` 0))
    (`KismetSystemLibrary.PrintString` "Local" true true (struct :`G` 0.66 :`B` 1.0 :`A` 1.0) 0.0)
    (else
      (`KismetSystemLibrary.PrintString` "Server" true true (struct :`G` 0.66 :`B` 1.0 :`A` 1.0) 0.0))))

(event `SetLaserMesh`
  (params (End :type "Vector Structure") (Start :type "Vector Structure"))
  (bind _returnvalue (- End Start))
  ;[0.2555 0.7775 1] updateLaserEvent
  (`SceneComponent.K2_SetWorldLocation` (`self.LaserScaleRoot`) Start false false)
  (`SceneComponent.K2_SetWorldRotation` (`self.LaserScaleRoot`) (`KismetMathLibrary.MakeRotFromZ` _returnvalue) false false)
  (`SceneComponent.SetWorldScale3D` (`self.LaserScaleRoot`) (`KismetMathLibrary.MakeVector` (`self.LaserSize`) 0.01 (* (`KismetMathLibrary.VSize` _returnvalue) 0.01))))

(event `UpdateOnServer`
  (params (HitLaserStart :type "Vector Structure") (HitLaserEnd :type "Vector Structure"))
  ;[0.2555 0.7775 1] updateLaserEvent
  (set `self.HitLaserStart` HitLaserStart)
  (set `self.HitLaserEnd` HitLaserEnd))

(event `UpdateLaser`
  (params (OffsetStartLocation :type "Vector Structure") (StartLocation :type "Vector Structure") (SetStartLocation :type Boolean) (hit :type "HitResult Structure"))
  ;[0.2555 0.7775 1] updateLaserEvent
  (`self.GetLaserLocations` (select `bool` SetStartLocation :`false` (select `bool` (`self.IsTouch`) :`false` (`PlayerController.GetHitResultUnderCursorForObjects` (`GameplayStatics.GetPlayerController` 0) (`|MakeArray` "ObjectTypeQuery1" "ObjectTypeQuery2" :!type "EObjectTypeQuery Enum") true) :`true` (`PlayerController.GetHitResultUnderFingerForObjects` (`GameplayStatics.GetPlayerController` 0) "Touch1" (`|MakeArray` "ObjectTypeQuery1" "ObjectTypeQuery2" :!type "EObjectTypeQuery Enum") true)) :`true` hit) OffsetStartLocation StartLocation))

(fn `GetLaserLocations`
  (params (Hit :type "HitResult Structure (by ref)") (OffsetStartLocation_ :type "Vector Structure") (StartLocation_ :type "Vector Structure") (SetStartLocation_ :type Boolean))
  (bind (_bblockinghit _binitialoverlap _time _distance _location) (`GameplayStatics.BreakHitResult` Hit))
  (bind _returnvalue (+ (select `bool` SetStartLocation_ :`false` (`SceneComponent.K2_GetComponentLocation` (`/Game/CollaborativeViewer/Blueprints/Pawn/BP_BasePawn.Camera` (cast `/Game/CollaborativeViewer/Blueprints/Pawn/BP_BasePawn` (`GameplayStatics.GetPlayerPawn` 0) :!pure true))) :`true` StartLocation_) OffsetStartLocation_))
  (set `self.HitLaserStart` _returnvalue)
  (set `self.HitLaserEnd` (select `bool` _bblockinghit :`false` _returnvalue :`true` _location)))

(fn `OnRep_HitLaserStart`)

(fn `UserConstructionScript`)